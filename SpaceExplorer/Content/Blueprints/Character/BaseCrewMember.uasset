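; Base crew member character that handles punching, health, walk speed and carried items.
; Punch triggers AttackComponent, whose hit event feeds CombatLogic to call CallHit on destroyable components or deal random damage to any other crew member.
; Damage lowers health and plays a pain sound, while Dead and EquipItemOnMesh are stubs, presumably for child overrides.
; Equipping drops the current item, flags the new one and shows a pickup notification.
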(event Custom|OnTargetHit
  (params (Hit%20Actor :type Actor%20Object%20Reference))
  ;[1 1 1] Subscribe to Target hit event of attack component
  (|CombatLogic Hit%20Actor))

(event Custom|TakeDamage_Event
  (params (Damage :type Float%20%28single-precision%29 :default 0.0))
  (CallFunction|UpdateHealth Damage))

(event EventBeginPlay
  ;[1 1 1] Subscribe to Target hit event of attack component
  (EventDispatchers|BindEventtoTargetHit (Variables|Default|GetAttackComponent) (delegate Custom|OnTargetHit)))

(fn ConstructionScript)

(fn Punch
  (if (not (Variables|State|GetIs%20Attacking))
    ;[1 1 1] Attack Animation
    (Variables|State|SetIs%20Attacking true)
    (Default|Attack (Variables|Default|GetAttackComponent))))

(fn HitDestroyableActor
  (params (actor :type Actor%20Object%20Reference))
  (bind _returnvalue (Actor|GetComponentsByClass actor "/Game/Blueprints/Components/DestroyableComponent.DestroyableComponent_C"))
  (return (> (Utilities|Array|Length _returnvalue) 0) (Utilities|Array|Get(acopy) _returnvalue)))

(fn HitEnemyCrewmember
  (params (actor :type Actor%20Object%20Reference))
  (bind _asbase_crew_member (Utilities|Casting|CastToBaseCrewMember actor))
  (return true _asbase_crew_member))

(fn Dead
  (return false))

(fn UpdateHealth
  (params (InputPin :type Float%20%28single-precision%29))
  (bind _audio (Variables|Default|GetAudio))
  ;[0.3077 1 0.2929] Update Health
  (Variables|Settings|Health|SetCurrent%20Health (- (Variables|Settings|Health|GetCurrent%20Health) InputPin))
  (Utilities|FlowControl|Sequence
    (:then_0
      (bind _returnvalue (Audio|Components|Audio|IsPlaying (Variables|Default|GetAudio)))
      (if (not _returnvalue)
        (Audio|Components|Audio|SetSound _audio (Variables|Sounds|GetPain))
        (Audio|Components|Audio|Play _audio 0.0)))
    (:then_1
      (Utilities|IsDead)
      (CallFunction|Dead)
      (return))))

(fn SetWalkSpeed
  (params (Max%20speed :type Float%20%28single-precision%29 :default 0.0))
  (Variables|/Script/Engine.CharacterMovementComponent|SetMaxWalkSpeed (Variables|Character|GetCharacterMovement) Max%20speed)
  (return))

(fn Equip
  (params (new%20item :type Base%20Equipable%20Object%20Reference))
  (Utilities|IsValid (Variables|Equipment|GetEquiped%20Item)
    (:Is%20Valid
      (|DropItem))
    (:Is%20Not%20Valid
      _))
  (|EquipItem new%20item))

(fn UseEquipedItem
  (bind _equiped_item (Variables|Equipment|GetEquiped%20Item))
  (if (and (Utilities|IsValid _equiped_item) (not (Variables|State|GetIs%20using%20equipment)))
    (Variables|State|SetIs%20using%20equipment true)
    (Default|Use _equiped_item)))

(fn EquipItemonMesh
  (return false))