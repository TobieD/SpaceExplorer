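; FuelDiscovery is a discovery Blueprint that rewards the player with ship fuel when unlocked.
; It overrides Unlock to add score, give the player ship a random fuel amount between MinFuel and MaxFuel, call the parent, and return a message.
; The message calls the random range node separately, so the reported amount can differ from the fuel added.
; Its event graph is empty.
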(event `self.ReceiveBeginPlay`)

(event `self.ReceiveActorBeginOverlap`
  (params (OtherActor :type "Actor Object Reference")))

(event `self.ReceiveTick`
  (params (DeltaSeconds :type "Float (single-precision)")))

(fn `Unlock`
  (returns (`Discovery info` :type Text))
  (bind _returnvalue (`KismetMathLibrary.RandomIntegerInRange` (`self.Min Fuel`) (`self.Max Fuel`)))
  (`/Game/Blueprints/General/Helpers.Add Score` 10)
  (`/Game/Blueprints/Ship/Ship.Add Fuel` (`/Game/Blueprints/General/Helpers.Get Player Ship`) _returnvalue)
  (`parent.Unlock`)
  (return (`|FormatText` "Found {x} fuel to power your ship" (`KismetTextLibrary.Conv_IntToText` _returnvalue))))

(fn `UserConstructionScript`
  (`parent.UserConstructionScript`))