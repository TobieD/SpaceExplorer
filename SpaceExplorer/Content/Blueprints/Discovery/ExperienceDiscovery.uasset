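; Discovery Blueprint that rewards the player's ship with a random amount of experience when unlocked.
; Unlock rolls a floored random value within a hardcoded range, grants it to the player ship, calls the parent Unlock and returns a formatted text reporting the award.
; The event graph is empty, and a leftover macro holds an unconnected roll based on MinXp and MaxXp.
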(event EventBeginPlay)

(event EventActorBeginOverlap
  (params (OtherActor :type Actor%20Object%20Reference)))

(event EventTick
  (params (DeltaSeconds :type Float%20%28single-precision%29)))

(fn ConstructionScript
  (|CallParentFunction))

(fn Unlock
  (bind _output_get (LocalVariables|Setexperience (Math|Conversions|ToFloat(Integer) (Math|Float|Floor (Math|Random|RandomFloatinRange 25.0 75.0)))))
  (Default|GrantExperience (CallFunction|GetPlayerShip) _output_get)
  (|CallParentFunction)
  (return (Utilities|Text|FormatText "Granted {XP} experience to ship" (Utilities|Text|ToText(Float) _output_get "HalfToEven"))))