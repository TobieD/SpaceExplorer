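; Discovery that, when unlocked, puts an enemy invader aboard the player's ship.
; Unlock spawns an EnemyCrewMember with the EnemyCrew_BT behavior tree just above a random ship tile, sets its AI state, calls the parent Unlock and returns a boarding message.
; GetRandomTile picks from the ship's ChildTiles using RandomInteger of length minus one, so the last tile is never chosen.
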(fn `Get Random Tile`
  (returns (Tile :type "/Game/Blueprints/Ship/Generation/ShipTile Object Reference"))
  (bind _childtiles (`/Game/Blueprints/Ship/Ship.ChildTiles` (`/Game/Blueprints/General/Helpers.Get Player Ship`)))
  (return (`KismetArrayLibrary.Array_Get` _childtiles (`KismetMathLibrary.RandomInteger` (- (`KismetArrayLibrary.Array_Length` _childtiles) 1)))))

(fn `Unlock`
  (returns (`Discovery info` :type Text))
  (bind _returnvalue (`AIBlueprintHelperLibrary.SpawnAIFromClass` "/Game/Blueprints/Character/Enemy/EnemyCrewMember.EnemyCrewMember_C" "/Game/Blueprints/Character/Enemy/EnemyCrew_BT.EnemyCrew_BT" (+ (`self.K2_GetActorLocation` (`self.Get Random Tile`)) (0.0 0.0 100.0))))
  (bind _asenemy_crew_member (cast `/Game/Blueprints/Character/Enemy/EnemyCrewMember` _returnvalue))
  (set `/Game/Blueprints/Character/Enemy/EnemyCrewMember.AI State` "NewEnumerator2" _asenemy_crew_member)
  (`parent.Unlock`)
  (return (`|FormatText` "An enemy has boarded your ship")))

(fn `UserConstructionScript`
  (`parent.UserConstructionScript`))