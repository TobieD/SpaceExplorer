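; An attack component that detects targets in front of its owning actor with a line trace.
; The Attack event traces for configured object types between computed ray positions and broadcasts the hit actor through the TargetHit dispatcher.
; A DebugMode flag enables timed trace drawing and prints the name of the hit target.
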(event `self.ReceiveTick`
  (params (DeltaSeconds :type "Float (single-precision)")))

(event `self.ReceiveInitializeComponent`)

(event `Attack`
  (bind _returnvalue (`self.GetOwner`))
  (bind _length (`self.Length`))
  (bind _returnvalue_2 (`Actor.K2_GetActorLocation` _returnvalue))
  ;[1 0.7855 0.2499] Raytrace infront of owner
  (bind (_outhit _returnvalue_3) (`KismetSystemLibrary.LineTraceSingleForObjects` :`Start` _returnvalue_2 :`End` (+ _returnvalue_2 (* (`KismetMathLibrary.GetForwardVector` (`Actor.K2_GetActorRotation` _returnvalue)) (`KismetMathLibrary.MakeVector` _length _length))) :`ObjectTypes` (`self.Object Types`) :`DrawDebugType` (`self.Debug mode Enabled`)))
  (if _returnvalue_3
    ;[1 0.17 0.17] Debug text
    (if (`self.Debug Mode`)
      (bind (_bblockinghit _time _location _normal _impactpoint _impactnormal _physmat _hitactor) (`GameplayStatics.BreakHitResult` _outhit))
      (`KismetSystemLibrary.PrintText` (`|FormatText` "hit target {t}" (`KismetTextLibrary.Conv_StringToText` (`KismetSystemLibrary.GetDisplayName` _hitactor)))))
    (`self.TargetHit` _hitactor)))

(fn `Debug mode Enabled`
  (returns (ReturnValue :type "KismetSystemLibrary.EDrawDebugTrace Enum"))
  (return (select `bool` (`self.Debug Mode`) :`true` "ForDuration" :!type "KismetSystemLibrary.EDrawDebugTrace Enum")))