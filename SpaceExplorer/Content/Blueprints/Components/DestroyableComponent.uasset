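; Actor component that makes its owner destroyable after a number of hits, with optional timed repair.
; On initialization it sets the hit count, binds to a Hit event and tags the owner.
; While enabled, each hit lowers the remaining count; at zero or below it fires Destroy and, if repairable, starts a Repair timer.
; Repair fires Repaired and restores base MaxHits, excluding any extra hits added through UpdateMaxHits.
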(event `self.ReceiveInitializeComponent`
  (`self.Update Max Hits` 0.0)
  (add `self.Hit` (delegate `Hit_Event`))
  (`KismetArrayLibrary.Array_Add` (`Actor.Tags` (`self.GetOwner`)) (`self.Tag`)))

(event `Hit_Event`
  (if (`self.Enabled`)
    ;[1 1 1] Lower hits needed
    (set `self.Remaining hits` (- (`self.Remaining hits`) 1.0))
    (if (`self.Is Destroyed`)
      (`self.Destroy`)
      (set `self.Destroyed` true)
      (if (`self.Can be repaired`)
        (`KismetSystemLibrary.K2_SetTimer` null "Repair" (`self.Repair Duration`))))))

(fn `Is Destroyed`
  (returns (Destroyed :type Boolean))
  (return (<= (`self.Remaining hits`) 0.0)))

(fn `Repair`
  (`self.Repaired`)
  (set `self.Remaining hits` (`self.Max hits`))
  (set `self.Destroyed` false))

(fn `Update Max Hits`
  (params (`New Max Hits` :type "Float (double-precision)" :default 0.0))
  (bind _output_get (set `self.Extra Hits` `New Max Hits`))
  (set `self.Remaining hits` (+ _output_get (`self.Max hits`))))