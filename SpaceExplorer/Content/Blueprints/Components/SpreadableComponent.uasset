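; Component that periodically spreads an effect from its parent actor to adjacent tiles, reporting each actor it finds through a FoundActor dispatcher.
; Start and Stop control a looping timer that probes four directions at a fixed tile offset, optionally with random skipping.
; An optional wall trace lets spreading pass only through clear space or open Doors.
; A downward trace then finds the neighboring actor, with optional debug drawing and text.
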(fn FindNextTile
  ;[1 1 1] Look in 4 Directions
  (CallFunction|TryFind 0.0 512.0)
  (CallFunction|TryFind 0.0 -512.0)
  (CallFunction|TryFind 512.0 0.0)
  (CallFunction|TryFind -512.0 0.0))

(fn Start
  (Utilities|Time|SetTimerbyFunctionName 0 "FindNextTile" (Variables|Settings|GetSpreadRate) true))

(fn Stop
  (Utilities|Time|ClearTimerbyFunctionName 0 "FindNextTile"))

(fn TryFind
  (params (X%20Offset :type Float%20%28single-precision%29 :default 0.0) (Y%20Offset :type Float%20%28single-precision%29))
  ;[0.2884 0.68 0.2152] Store as local
  (LocalVariables|SetX X%20Offset)
  (LocalVariables|SetY Y%20Offset)
  ;[1 0.1 0.1] RAndomize the spreading
  (if (Variables|Settings|GetRandomize)
    (if (< (Math|Random|RandomIntegerinRange 0 5) 2)
      (if (Variables|Settings|GetCheck%20Walls) :!label _label
        (|CanPassthrough
          (:Yes
            _)))
      (|FindActor))
    (else
      (goto _label))))