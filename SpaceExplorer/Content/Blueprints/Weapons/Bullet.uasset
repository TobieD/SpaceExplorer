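; Homing bullet actor that flies toward a Target actor and bursts on reaching it.
; Each Tick it steps along the direction to the target by Speed, without sweep or delta-time scaling, and tests proximity by distance rather than collision.
; On arrival a Destroyed flag blocks retriggering while it activates the ExplodeP effect, hides the cube and destroys itself after a delay; it applies no damage.
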(event `self.ReceiveBeginPlay`
  (`ActorComponent.SetActive` (`self.Explode_P`) false false))

(event `self.ReceiveTick`
  (params (DeltaSeconds :type "Float (single-precision)"))
  (bind _returnvalue (`self.K2_GetActorLocation`))
  (bind _target (`self.Target`))
  (bind _returnvalue_2 (`self.K2_GetActorLocation` _target))
  (`/Engine/EditorBlueprintResources/StandardMacros.IsValid` _target
    (:`Is Valid`
      (`self.K2_SetActorLocation` (+ _returnvalue (* (`KismetMathLibrary.Normal` (- _returnvalue_2 _returnvalue)) (`self.speed`))))
      (if (and (not (`self.Destroyed`)) (< (`KismetMathLibrary.VSize` (- (`self.K2_GetActorLocation`) _returnvalue_2)) 50.0))
        (set `self.Destroyed` true)
        (`ActorComponent.Activate` (`self.Explode_P`) true)
        (`SceneComponent.SetVisibility` (`self.Cube`) false false)
        (`KismetSystemLibrary.Delay` 5.0)
        (`self.K2_DestroyActor`)))))

(fn `UserConstructionScript`)