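; Base ship weapon that targets tiles on a ship and damages that ship when fired.
; Tick raycasts under the cursor while targeting and stops the looping cooldown timer once the weapon is ready.
; Fire checks ammo, cooldown and enemy state, applies damage immediately, calls a stub effect hook, then spawns a bullet and notification.
; The ship's WeaponSystem boosts cooldown recovery and, when maxed, sometimes waives ammo cost.
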(event `self.ReceiveTick`
  (params (DeltaSeconds :type "Float (single-precision)"))
  (bind (_bblockinghit _time _location _normal _impactpoint _impactnormal _physmat _hitactor) (`GameplayStatics.BreakHitResult` (`PlayerController.GetHitResultUnderCursorForObjects` (`GameplayStatics.GetPlayerController` 0) (`|MakeArray` "ObjectTypeQuery1" :!type "EngineTypes.EObjectTypeQuery Enum") true)))
  (if (`self.CanFire`)
    (`KismetSystemLibrary.K2_ClearTimer` null "Reduce Cooldown"))
  (if (`self.FindTarget`)
    (`self.K2_SetActorLocation` (`/Game/Blueprints/General/GameState_Ftl.WeaponTarget` (`/Game/Blueprints/General/Helpers.Get Game State FTL`)) _location false)
    (bind _asship_tile (cast `/Game/Blueprints/Ship/Generation/ShipTile` _hitactor))
    (set `self.Target` _asship_tile)))

(fn `Apply Weapon Effect`
  (returns (Fired :type Boolean))
  (return false))

(fn `Fire`
  (bind _returnvalue (`self.Calculate Damage`))
  (bind _parent_ship (`self.Parent Ship`))
  (bind _weaponbehaviour (`self.WeaponBehaviour`))
  (bind _parent_ship_2 (`self.Parent Ship`))
  (bind _parentship (`/Game/Blueprints/Ship/Generation/ShipTile.ParentShip` (`self.Target`)))
  ;[0.4169 0.6991 1] Check if target is found and valid
  (`/Engine/EditorBlueprintResources/StandardMacros.IsValid` (`self.Target`)
    (:`Is Valid`
      ;[1 0.115 0.115] Check if weapon can be fired
      (if (and (`self.HasAmmo`) (`self.CanFire`) (`/Game/Blueprints/Ship/EnemyShip.Is Active` (`/Game/Blueprints/General/Helpers.Get Enemy Ship`)))
        (`|ExecutionSequence`
          (:`then_0`
            (`/Engine/EditorBlueprintResources/StandardMacros.IsValid` _parent_ship
              (:`Is Valid`
                (for _array_element (`/Game/Blueprints/Ship/Ship.AvailableSystems` _parent_ship)
                  (bind _asweapon_system (cast `/Game/Blueprints/Systems/WeaponSystem` _array_element))
                  (set `self.WeaponBehaviour` _asweapon_system)
                  (break))
                (if (>= (`/Game/Blueprints/Systems/BaseSystem.Current Level` _weaponbehaviour) (`/Game/Blueprints/Systems/BaseSystem.Max Level` _weaponbehaviour))
                  (if (not (<= (`KismetMathLibrary.RandomInteger` 5) 0))
                    (`/Game/Blueprints/Ship/Ship.Take Ammo` (`self.Parent Ship`) (`self.Required Ammo`) :!label _label))
                  (else
                    (goto _label)))
                ;[0.6411 1 0.397] Reset Cooldown + start timer
                (set `self.CurrentCooldown` 0.0)
                (`KismetSystemLibrary.K2_SetTimer` null "Reduce Cooldown" 1.0 true))))
          (:`then_1`
            ;[0 1 0.363] Damage the enemy
            (`/Game/Blueprints/Ship/Ship.Take Damage` _parentship (`KismetMathLibrary.Conv_IntToDouble` _returnvalue))
            (`self.Apply Weapon Effect`)
            ;[0.09557 0.7282 1] Spawn a bullet
            (`/Engine/EditorBlueprintResources/StandardMacros.IsValid` _parent_ship_2
              (:`Is Valid`
                (`|SpawnActorFromClass` "/Game/Blueprints/Weapons/Bullet.Bullet_C" (`KismetMathLibrary.MakeTransform` (+ (.location (`self.GetTransform` _parent_ship_2)) (0.0 0.0 200.0)) (.rotation (`self.GetTransform` _parent_ship_2)) (.scale (`self.GetTransform` _parent_ship_2))) false (`self.BulletMesh`) (`self.Target`))
                (`/Game/Blueprints/General/Helpers.Notify` (`|FormatText` "{ship} hit for {dmg}!" (`KismetTextLibrary.Conv_StringToText` (`KismetSystemLibrary.GetDisplayName` _parentship)) (`KismetTextLibrary.Conv_IntToText` _returnvalue)) 1.0 "NewEnumerator2")))))))))

(fn `OnCooldown`
  (returns (OnCooldown :type Boolean))
  (return (not (`self.CanFire`))))

(fn `Reduce Cooldown`
  (set `self.CurrentCooldown` (+ (`self.CurrentCooldown`) (+ (`self.CooldownRestoreRate`) (`/Game/Blueprints/Systems/WeaponSystem.Bonus Cooldown restore rate` (`self.WeaponBehaviour`))))))

(fn `UserConstructionScript`)