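; Weapon inventory for a ship that holds equipped weapons, tracks the selected one and refreshes the HUD as the loadout changes.
; SpawnWeapon spawns a random class from PossibleWeapons and passes it to AddWeapon, which equips and selects it or opens a replace-weapon widget.
; Replace swaps a weapon in at the given index and destroys the old one.
; Selection only flags the new weapon, while Tick clears the flag on all others.
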(event EventTick
  (params (DeltaSeconds :type Float%20%28single-precision%29))
  (for _array_element (Variables|Weapons|GetEquipedWeapons)
    (if (!= _array_element (Variables|Weapons|GetSelectedWeapon))
      (Variables|/Game/Blueprints/Weapons/BaseWeapon.BaseWeapon_C|SetSelected _array_element false))))

(event EventBeginPlay
  (Default|RefreshWeaponUI (CallFunction|GetHUD)))

(fn ConstructionScript)

(fn AddWeapon
  (params (newWeapon :type Base%20Weapon%20Object%20Reference))
  (bind _output_get (LocalVariables|Setweapon_Local newWeapon))
  (Utilities|IsValid _output_get
    (:Is%20Valid
      (Utilities|FlowControl|Sequence
        (:then_0
          (Variables|/Game/Blueprints/Weapons/BaseWeapon.BaseWeapon_C|SetParent%20Ship (LocalVariables|Getweapon_Local) (Variables|Default|GetParent%20Ship))
          ;[1 1 1] Add or Replace Weapon
          (if (Utilities|CanAddWeapon)
            (|AddWeapon)
            (else
              (|ReplaceWeapon))))
        (:then_1
          ;[1 1 1] Update UI
          (Default|RefreshWeaponUI (CallFunction|GetHUD)))))))

(fn SelectWeapon
  (params (index :type Integer :default 0))
  (Utilities|ToggleSelected (Utilities|Array|Get(acopy) (Variables|Weapons|GetEquipedWeapons) index)))

(fn Replace
  (params (Index%20to%20replace :type Integer :default 0) (new%20weapon :type Base%20Weapon%20Object%20Reference))
  (bind _equipedweapons (Variables|Weapons|GetEquipedWeapons))
  ;[1 1 1] Set Local Variables
  (LocalVariables|Setindex Index%20to%20replace)
  (LocalVariables|SetWeapon_Local new%20weapon)
  (LocalVariables|SetReplacedWeapon (Utilities|Array|Get(acopy) _equipedweapons (LocalVariables|Getindex)))
  ;[1 1 1] Remove Weapon At Index
  (Utilities|Array|RemoveIndex _equipedweapons (LocalVariables|Getindex))
  ;[1 1 1] Insert New Weapon
  (Utilities|Array|Insert _equipedweapons (LocalVariables|GetWeapon_Local) (LocalVariables|Getindex))
  (Actor|DestroyActor (LocalVariables|GetReplacedWeapon))
  (Variables|Default|SetReplaceUIOpen false)
  ;[1 1 1] Update UI
  (Default|RefreshWeaponUI (CallFunction|GetHUD)))

(fn SpawnWeapon
  (bind _possibleweapons (Variables|Weapons|GetPossibleWeapons))
  (bind _returnvalue (Game|SpawnActorfromClass (Utilities|Array|Get(acopy) _possibleweapons (Math|Random|RandomIntegerinRange 0 (- (Utilities|Array|Length _possibleweapons) 1))) (Math|Transform|MakeTransform "0, 0, 0") true 0))
  (Utilities|IsValid _returnvalue
    (:Is%20Valid
      (CallFunction|AddWeapon _returnvalue)
      (return (Variables|/Game/Blueprints/Weapons/BaseWeapon.BaseWeapon_C|GetName _returnvalue)))))