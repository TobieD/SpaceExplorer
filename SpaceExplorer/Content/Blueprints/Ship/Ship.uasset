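; Ship actor that tracks hull, shield, fuel, ammo, engine power and crew, with reduced damage for the player's ship.
; BeginPlay spawns randomly named crew on unique owned tiles, creates a weapon collection and registers the ship's workstation behaviours.
; Travel spends fuel and engine power, which a looping timer restores, while damage hits active shields or hull.
; Tick calls DestroyShip when hull, crew or fuel runs out, though it and SpawnCrewmember are stubs here.
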(event EventTick
  (params (DeltaSeconds :type Float%20%28single-precision%29))
  ;[0.825 0.06188 0.06188] Check Ship State
  (Utilities|HasHullRemaining
    (:True
      (Utilities|HasCrewRemaining
        (:True
          (Utilities|HasFuel
            (:False
              _)))
        (:False
          _)))
    (:False
      _))
  (Damage|DestroyShip))

(event EventBeginPlay
  (|Initialization))

(fn ConstructionScript)

(fn SpawnCrew
  (|FindChildTiles
    (:Found
      ;[0.09557 0.7282 1] Add the specified amount of crewmembers
      (for _index (range 1 (Variables|Crew|GetCrew%20Size))
        (Crew|AddCrewMember))
      (return))))

(fn FindUniqueSpawn
  (params (Array :type Array%20of%20Actor%20Object%20References))
  (LocalVariables|SetActorArray Array)
  ;[1 0.4788 0.11] Find a random transform based on an actor array
  (bind _new_transform (CallFunction|RandomTransformfromList (LocalVariables|GetActorArray)))
  (LocalVariables|Setnew%20transform _new_transform)
  (while (Utilities|Array|ContainsItem (Variables|Crew|Spawn|GetCrewStartPositions) (LocalVariables|Getnew%20transform))
    ;[1 0.4788 0.11] Find a new unique transform
    (bind _new_transform_2 (CallFunction|RandomTransformfromList (LocalVariables|GetActorArray)))
    (LocalVariables|Setnew%20transform _new_transform_2))
  ;[1 0.4788 0.11] Add the new transform to the list of used transforms
  (Utilities|Array|Add (Variables|Crew|Spawn|GetCrewStartPositions) (LocalVariables|Getnew%20transform))
  (return (Math|Transform|MakeTransform (+ "0,0.000000,100.000000" (.Location (Math|Transform|BreakTransform (LocalVariables|Getnew%20transform)))) (.Rotation (Math|Transform|BreakTransform (LocalVariables|Getnew%20transform))) (.Scale (Math|Transform|BreakTransform (LocalVariables|Getnew%20transform))))))

(fn HasFullShields
  (return (not (< (Variables|ShipSystem|Shield|GetCurrent%20Shield%20) (Variables|ShipSystem|Shield|GetMax%20Shield)))))

(fn AddCrewMember
  ;[1 0.4788 0.11] Find unique spawn location
  (bind _result (Crew|FindUniqueSpawn (Variables|ShipSystem|General|GetChildTiles)))
  ;[0.2884 0.68 0.2152] Find a random name for the crewmember
  (bind _new_text (CallFunction|RandomTextfromList (Variables|Crew|Spawn|GetCrewNames)))
  (bind _crewmember (Crew|Spawn|SpawnCrewmember _new_text _result))
  (Utilities|IsValid _crewmember
    (:Is%20Valid
      ;[0.09557 0.7282 1] Add the member to the crew
      (Utilities|Array|Add (Variables|Crew|Spawn|GetCrewList) _crewmember)
      (return _crewmember))))

(fn RestoreEnginePower
  (bind _engine_restore_rate (Variables|ShipSystem|Engine|GetEngine%20Restore%20Rate))
  (Variables|ShipSystem|Engine|SetCurrent%20Engine%20Power (Math|Float|Clamp(Float) (+ (Variables|ShipSystem|Engine|GetCurrent%20Engine%20Power) (+ _engine_restore_rate (* _engine_restore_rate (Variables|ShipSystem|Engine|GetBonus%20Engine%20Recharge)))) 0.0 (Variables|ShipSystem|Engine|GetMax%20Engine%20Power))))

(fn Travel
  (Utilities|Time|ClearTimerbyFunctionName 0 "RestoreEnginePower")
  (Variables|ShipSystem|Engine|SetCurrent%20Engine%20Power 0.0) ; Reset to 0
  (Utilities|Time|SetTimerbyFunctionName 0 "RestoreEnginePower" 1.5 true)
  (Variables|ShipSystem|Engine|SetFuel (- (Variables|ShipSystem|Engine|GetFuel) 1)))

(fn CanTravel
  (return (and (>= (Variables|ShipSystem|Engine|GetCurrent%20Engine%20Power) (Variables|ShipSystem|Engine|GetMax%20Engine%20Power)) (> (Variables|ShipSystem|Engine|GetFuel) 0))))

(fn RemoveCrewMember
  (params (CrewMember :type Base%20Crew%20Member%20Object%20Reference))
  ;[0.09557 0.7282 1] Remove Crew from the crewList
  (bind _returnvalue (Utilities|Array|RemoveItem (Variables|Crew|Spawn|GetCrewList) CrewMember))
  (return _returnvalue))

(fn TakeDamage
  (params (Damage :type Float%20%28single-precision%29))
  ;[1 1 1] Player has additional defense
  (if (== (CallFunction|GetPlayerShip) self)
    (LocalVariables|Setdmg (* Damage 0.8))
    (else
      (LocalVariables|Setdmg Damage)))
  ;[1 0.1 0.1] Damage shield or hull based on shields
  (Utilities|HasShields
    (:True
      (|DamageShield))
    (:False
      (|DamageHull))))

(fn AddFuel
  (params (New%20Fuel :type Integer :default 0))
  (Variables|ShipSystem|Engine|SetFuel (+ New%20Fuel (Variables|ShipSystem|Engine|GetFuel))))

(fn DestroyShip
  (return true))

(fn TakeAmmo
  (params (Amount :type Integer :default 0))
  (Variables|ShipSystem|Weapon|SetCurrent%20Ammo (Math|Integer|Clamp(Integer) (- (Variables|ShipSystem|Weapon|GetCurrent%20Ammo) Amount) 0 (Variables|ShipSystem|Weapon|GetMax%20Ammo))))

(fn GiveAmmo
  (params (Amount :type Integer :default 0))
  (Variables|ShipSystem|Weapon|SetCurrent%20Ammo (Math|Integer|Clamp(Integer) (+ (Variables|ShipSystem|Weapon|GetCurrent%20Ammo) Amount) 0 (Variables|ShipSystem|Weapon|GetMax%20Ammo))))

(fn SpawnCrewmember
  (params (Name :type Text) (Spawn :type Transform))
  (return 0))

(fn FindSystem
  (params (System :type ESystem%20Enum :default "NewEnumerator0"))
  (for _array_element (Variables|Default|GetAvailableSystems)
    (if (== (Variables|/Game/Blueprints/Ship/Interactables/WorkStation.WorkStation_C|GetActive%20Behaviour (Variables|/Game/Blueprints/Systems/BaseSystem.BaseSystem_C|GetWorkStation _array_element)) System)
      (return (Variables|/Game/Blueprints/Ship/Interactables/WorkStation.WorkStation_C|GetWorkBehaviour (Variables|/Game/Blueprints/Systems/BaseSystem.BaseSystem_C|GetWorkStation _array_element))))))

(fn Repair
  (params (Amount :type Float%20%28single-precision%29))
  (Variables|ShipSystem|Hull|SetCurrent%20Hull (Math|Float|Clamp(Float) 0.0 (+ Amount (Variables|ShipSystem|Hull|GetCurrent%20Hull)) (Variables|ShipSystem|Hull|GetMax%20Hull))))