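; Enemy ship Blueprint that fights the player's ship, built on a parent ship class with tiles, crew and systems.
; It registers with the game state and starts hidden; Spawn restores hull and tiles, enables crew AI and re-tasks random crew.
; Attacks, also bound to a debug F key, fire a weapon at a random player tile.
; Destruction grants random experience, restores ambient sound, stops crew AI and hides the reusable ship after a delay.
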(event EventBeginPlay
  (|CallParentFunction)
  (|CreateEnemyShip))

(event EventTick
  (params (DeltaSeconds :type Float%20%28single-precision%29))
  (if (Variables|ShipSystem|General|GetIs%20Active)
    (|CallParentFunction DeltaSeconds)))

(event Input|KeyboardEvents|F
  (:Pressed
    (Development|PrintString "Attack Player")
    (CallFunction|AttackPlayerShip)))

(fn ConstructionScript
  (|CallParentFunction))

(fn Spawn
  (bind _crewlist (Variables|Default|GetCrewList))
  (Variables|ShipSystem|General|SetIs%20Active true)
  ;[0.2884 0.68 0.2152] Full Health
  (Variables|Default|SetCurrent%20Hull (Variables|Default|GetMax%20Hull))
  (Spawning|SetVisiblity true)
  ;[0.09557 0.7282 1] Reset all tiles to normal state
  (for _array_element (Variables|Default|GetChildTiles)
    (Default|SetTileState _array_element "NewEnumerator0")
    (for _array_element_2 _crewlist
      (bind _asenemy_crew_member (Utilities|Casting|CastToEnemyCrewMember _array_element_2))
      (Default|ToggleAI _asenemy_crew_member true))
    ;[1 1 1] Randomly enable 1 to attack the player
    (bind _asenemy_crew_member_2 (Utilities|Casting|CastToEnemyCrewMember (Utilities|Array|Get(acopy) _crewlist (Math|Random|RandomInteger (Utilities|Array|Length _crewlist)))))
    (Variables|/Game/Blueprints/Character/Enemy/EnemyCrewMember.EnemyCrewMember_C|SetAI%20State _asenemy_crew_member_2 "NewEnumerator1")))

(fn SetVisiblity
  (params (Visible :type Boolean :default false))
  (LocalVariables|Setnew%20visibility Visible)
  ;[1 0.9141 0.25] Change tiles visibility
  (for _array_element (Variables|Default|GetChildTiles)
    (Default|ToggleVisibility _array_element (LocalVariables|Getnew%20visibility)))
  ;[1 0.9141 0.25] Change crew visibility
  (for _array_element_2 (Variables|Default|GetCrewList)
    (bind _asenemy_crew_member (Utilities|Casting|CastToEnemyCrewMember _array_element_2))
    (Rendering|SetVisibility _asenemy_crew_member (LocalVariables|Getnew%20visibility) true))
  ;[1 0.7855 0.2499] Hide Workstations
  (for _array_element_3 (Variables|Default|GetAvailableSystems)
    (Rendering|SetVisibility (Variables|/Game/Blueprints/Systems/BaseSystem.BaseSystem_C|GetWorkStation _array_element_3) (LocalVariables|Getnew%20visibility) true)))

(fn DestroyShip
  (Variables|ShipSystem|General|SetIs%20Active false)
  (Default|GrantExperience (CallFunction|GetPlayerShip) (Math|Conversions|ToFloat(Integer) (Math|Float|Floor (Math|Random|RandomFloatinRange 5e+01 1e+02))))
  (Utilities|Time|SetTimerbyFunctionName 0 "DelayedDestroy" 5.0)
  ;[0.2699 0.5609 1] Back to standard sound
  (Audio|Components|Audio|SetSound (Variables|/Game/Blueprints/General/GameState_Ftl.GameState_Ftl_C|GetBackgroundSound (CallFunction|GetGameStateFTL)) "/Game/Sounds/Ambience/Ship_Ambience_Cue.Ship_Ambience_Cue")
  (for _array_element (Variables|Default|GetCrewList)
    (bind _asenemy_crew_member (Utilities|Casting|CastToEnemyCrewMember _array_element))
    (Default|ToggleAI _asenemy_crew_member false))
  (return true))

(fn SwitchCeiling
  (params (Visibility :type Boolean :default false))
  (if (Variables|ShipSystem|General|GetIs%20Active)
    (for _array_element (Variables|Default|GetChildTiles)
      (Rendering|SetVisibility _array_element Visibility true))))

(fn CheckShield
  (params (shield%20percentage :type Float%20%28single-precision%29 :default 0.0))
  (return (select (> shield%20percentage (Variables|Default|GetCurrent%20Shield%20)) true false)))

(fn SpawnCrewmember
  (params (Name :type Text) (Spawn :type Transform))
  (bind (_location _rotation) (Math|Transform|BreakTransform Spawn))
  (bind _returnvalue (AI|SpawnAIFromClass "/Game/Blueprints/Character/Enemy/EnemyCrewMember.EnemyCrewMember_C" "/Game/Blueprints/Character/Enemy/EnemyCrew_BT.EnemyCrew_BT" _location _rotation false))
  (bind _asenemy_crew_member (Utilities|Casting|CastToEnemyCrewMember _returnvalue))
  (Variables|/Game/Blueprints/Character/BaseCrewMember.BaseCrewMember_C|SetParent%20Ship _asenemy_crew_member self)
  (Variables|/Game/Blueprints/Character/BaseCrewMember.BaseCrewMember_C|SetName _asenemy_crew_member Name)
  (return _asenemy_crew_member))

(fn AttackPlayerShip
  (bind _player_ship (CallFunction|GetPlayerShip))
  (bind _childtiles (Variables|/Game/Blueprints/Ship/Ship.Ship_C|GetChildTiles _player_ship))
  (if (Variables|ShipSystem|General|GetIs%20Active)
    ;[1 0.17 0.17] Find a weapon not on cooldown
    (bind _array_element (Utilities|Array|ForEachLoopwithBreak (Variables|/Game/Blueprints/Weapons/WeaponCollection.WeaponCollection_C|GetEquipedWeapons (Variables|Default|GetWeaponSystem)) :!label _label)
      (:LoopBody
        (bind _oncooldown (Default|OnCooldown _array_element))
        (if (not _oncooldown)
          (goto _label Break)))
      (:Completed
        (Variables|/Game/Blueprints/Weapons/BaseWeapon.BaseWeapon_C|SetTarget _array_element (Utilities|Array|Get(acopy) _childtiles (Math|Random|RandomInteger (- (Utilities|Array|Length _childtiles) 1))))
        (Default|Fire _array_element)))))

(fn DelayedDestroy
  (bind _found_system (Default|FindSystem (CallFunction|GetPlayerShip) "NewEnumerator2"))
  (bind _asweapon_system (Utilities|Casting|CastToWeaponSystem _found_system))
  (Default|FinishWorkingEvent _asweapon_system)
  (Spawning|SetVisiblity false))