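; The player's ship in an FTL-style game, a child ship Blueprint whose destruction loses the game.
; On BeginPlay it places the player's character on a tile as named crew and registers with the game state.
; Input cycles possession through the crew list, refreshing the HUD, and selects or fires WeaponSystem weapons.
; It also tracks experience, score on gains and skill points; an insta-kill debug weapon hook is left unconnected.
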(event EventBeginPlay
  (|CallParentFunction)
  (|SpawnPlayer)
  (|SetupInput+HUD))

(event EventTick
  (params (DeltaSeconds :type Float%20%28single-precision%29))
  (|CallParentFunction DeltaSeconds))

(event Input|ActionEvents|InputActionSwitchCrew
  ;[0.4615 1 0.7188] Switch through crew members
  (:Pressed
    (Crew|SwitchCrewMember)))

(event Input|ActionEvents|InputActionSelectTarget
  (bind _weaponsystem (Variables|Default|GetWeaponSystem))
  (bind _selectedweapon (Variables|/Game/Blueprints/Weapons/WeaponCollection.WeaponCollection_C|GetSelectedWeapon _weaponsystem))
  (:Pressed
    ;[0.4615 1 0.7188] Fire Weapon
    (Utilities|IsValid _weaponsystem
      (:Is%20Valid
        (Utilities|IsValid _selectedweapon
          (:Is%20Valid
            (Default|Fire _selectedweapon)))))))

(event Input|ActionEvents|InputActionSelectFirstWeapon
  ;[0.4615 1 0.7188] Weapon Swapping
  (:Pressed
    (|SelectWeapon)))

(event Input|ActionEvents|InputActionSelectFourthWeapon
  ;[0.4615 1 0.7188] Weapon Swapping
  (:Pressed
    (|SelectWeapon) ; enters at Weapon 4
  ))

(event Input|ActionEvents|InputActionSelectSecondWeapon
  ;[0.4615 1 0.7188] Weapon Swapping
  (:Pressed
    (|SelectWeapon) ; enters at Weapon 2
  ))

(event Input|ActionEvents|InputActionSelectThirdWeapon
  ;[0.4615 1 0.7188] Weapon Swapping
  (:Pressed
    (|SelectWeapon) ; enters at Weapon 3
  ))

(fn ConstructionScript
  (|CallParentFunction))

(fn SwitchCrewMember
  (bind _returnvalue (Game|GetPlayerController 0))
  ;[0.09557 0.7282 1] Select next crew member
  (bind _output_get (Variables|Default|SetCrewIndex (Utilities|GetNextCrewmember)))
  (bind _output_get_2 (Variables|Default|SetActive%20CrewMember (Utilities|Array|Get(acopy) (Variables|Default|GetCrewList) _output_get)))
  ;[0.4615 1 0.7188] Posses the new crew member
  (Pawn|Possess _returnvalue _output_get_2)
  ;[0.09557 0.7282 1] Posses event on CrewController
  (bind _asplayer_crew_controller (Utilities|Casting|CastToPlayerCrewController _returnvalue))
  (Default|OnPosseses _asplayer_crew_controller)
  (Crew|UpdateCrewUI))

(fn UpdateCrewUI
  (Default|RefreshCrewUI (Variables|/Game/Blueprints/General/GameState_Ftl.GameState_Ftl_C|GetPlayerHud (CallFunction|GetGameStateFTL))))

(fn RemoveCrewMember
  (params (CrewMember :type Base%20Crew%20Member%20Object%20Reference))
  (LocalVariables|Setcrewmember%20Local CrewMember)
  ;[0.09557 0.7282 1] Switch to next crewmember
  (if (== (Variables|Default|GetActive%20CrewMember) (LocalVariables|Getcrewmember%20Local))
    (Crew|SwitchCrewMember))
  (bind _succes (|CallParentFunction (LocalVariables|Getcrewmember%20Local)))
  (Crew|UpdateCrewUI)
  (return _succes))

(fn GrantExperience
  (params (Experience :type Float%20%28single-precision%29 :default 0.0))
  (LocalVariables|Setnew%20experience Experience)
  (if (>= (+ (LocalVariables|Getnew%20experience) (Variables|Leveling|GetCurrent%20Experience)) (Variables|Leveling|GetMax%20Experience))
    (Leveling|LevelUp (LocalVariables|Getnew%20experience))
    (CallFunction|AddScore (Math|Float|Floor (LocalVariables|Getnew%20experience)))
    (else
      ;[0.2884 0.68 0.2152] Add Experience
      (Variables|Leveling|SetCurrent%20Experience (+ (LocalVariables|Getnew%20experience) (Variables|Leveling|GetCurrent%20Experience))))))

(fn LevelUp
  (params (New%20Experience :type Float%20%28single-precision%29 :default 0.0))
  (CallFunction|AddScore (Math|Float|Floor (/ (Variables|Leveling|GetMax%20Experience) 2.0)))
  ;[0.2884 0.68 0.2152] Calculate remainder Xp
  (LocalVariables|Setremainder (- New%20Experience (Variables|Leveling|GetMax%20Experience)))
  ;[0.2884 0.68 0.2152] Level up
  (Variables|Leveling|SetCurrent%20Skillpoints (+ (Variables|Leveling|GetCurrent%20Skillpoints) 1))
  ;[0.2884 0.68 0.2152] Increase Max Experience
  (Variables|Leveling|SetMax%20Experience (+ (Variables|Leveling|GetMax%20Experience) (* (Variables|Leveling|GetCurrent%20Skillpoints) (Variables|Leveling|GetMax%20Experience))))
  (CallFunction|Notify "Leveled up" 2.0 "NewEnumerator0"))

(fn DestroyShip
  ;[1 0.9141 0.25] Lose the game
  (Default|Lose (CallFunction|GetGameModeFTL))
  (return true))

(fn CheckShieldPercentage
  (params (Check%20Percentage :type Float%20%28single-precision%29 :default 0.0))
  (return (select (> Check%20Percentage (Variables|Default|GetCurrent%20Shield%20)) true false)))

(fn GrantSkillpoint
  (Variables|Leveling|SetCurrent%20Skillpoints (Math|Integer|Clamp(Integer) (+ (Variables|Leveling|GetCurrent%20Skillpoints) 1) 0 99)))

(fn SpendSkillpoint
  (Variables|Leveling|SetCurrent%20Skillpoints (Math|Integer|Clamp(Integer) (- (Variables|Leveling|GetCurrent%20Skillpoints) 1) 0 99)))

(fn CanSpendSkillpoint
  (return (> (Variables|Leveling|GetCurrent%20Skillpoints) 0)))

(fn SpawnCrewmember
  (params (Name :type Text) (Spawn :type Transform))
  (bind _returnvalue (Game|SpawnActorfromClass "/Game/Blueprints/Character/Player/PlayerCrewMember.PlayerCrewMember_C" Spawn false Name self 0))
  (return _returnvalue))