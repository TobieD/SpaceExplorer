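; BaseEquipable is a base actor for items that a crew member can pick up and equip through an interact input.
; A radius-adjustable sphere trigger stores an overlapping BaseCrewMember and toggles the actor's input while the item is unequipped.
; Interacting passes the item to that crew member's Equip and disables further interaction.
; A widget is linked to the item, and a looping timer yaws it toward the player character.
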(event `InputAction|Interact`
  (:`Pressed`
    (`self.Interact`)))

(event `self.InteractTrigger.OnComponentBeginOverlap`
  (params (OtherActor :type "Actor Object Reference") (OtherComp :type "PrimitiveComponent Object Reference") (OtherBodyIndex :type Integer) (bFromSweep :type Boolean) (SweepResult :type "EngineTypes.HitResult Structure (by ref)"))
  (bind _debug (`self.Debug`))
  ;[1 1 1] Trigger Events
  (if (not (`self.IsEquiped`))
    (bind _asbase_crew_member (cast `/Game/Blueprints/Character/BaseCrewMember` OtherActor))
    (set `self.Interact Actor` _asbase_crew_member)
    (`self.Adjust Interaction` true)
    (`KismetSystemLibrary.PrintString` "Interaction Enabled" _debug _debug)))

(event `Always Face Player`
  (bind _interacttext (`self.InteractText`))
  (`SceneComponent.K2_SetWorldRotation` _interacttext (`KismetMathLibrary.MakeRot` 0.0 (+ (.yaw (`KismetMathLibrary.FindLookAtRotation` (`SceneComponent.K2_GetComponentLocation` (`GameplayStatics.GetPlayerCharacter` 0)) (`SceneComponent.K2_GetComponentLocation` _interacttext))) 90.0) 90.0) false))

(event `self.ReceiveBeginPlay`
  (add `self.Interact` (delegate `OnInteract`))
  (bind _asequipable_text (cast `/Game/Blueprints/HUD/WidgetExtensions/EquipableText` (`WidgetComponent.GetUserWidgetObject` (`self.InteractText`))))
  (set `/Game/Blueprints/HUD/WidgetExtensions/EquipableText.Owner` self _asequipable_text)
  (`KismetSystemLibrary.K2_SetTimerDelegate` (delegate `Always Face Player`) 0.1 true))

(event `self.InteractTrigger.OnComponentEndOverlap`
  (params (OtherActor :type "Actor Object Reference") (OtherComp :type "PrimitiveComponent Object Reference") (OtherBodyIndex :type Integer))
  (bind _debug (`self.Debug`))
  ;[1 1 1] Trigger Events
  (if (not (`self.IsEquiped`))
    (`self.Adjust Interaction` false)
    (set `self.Interact Actor` null)
    (`KismetSystemLibrary.PrintString` "Interaction Disabled" _debug _debug)))

(event `OnInteract`
  (bind _interact_actor (`self.Interact Actor`))
  (bind _debug (`self.Debug`))
  (if (not (`self.IsEquiped`))
    (`/Engine/EditorBlueprintResources/StandardMacros.IsValid` _interact_actor
      (:`Is Valid`
        (bind _output_get (set `self.Equip Actor` _interact_actor))
        (`/Game/Blueprints/Character/BaseCrewMember.Equip` _output_get self)
        (`self.Adjust Interaction` false)
        (`KismetSystemLibrary.PrintString` "Interaction" _debug _debug)))))

(fn `Adjust Interaction`
  (params (`Enable Interaction` :type Boolean :default false))
  (bind _returnvalue (`GameplayStatics.GetPlayerController` 0))
  (bind _output_get (set `self.Allow interaction` `Enable Interaction`))
  (if _output_get
    (`self.EnableInput` _returnvalue)
    (else
      (`self.DisableInput` _returnvalue))))

(fn `Use`
  (returns (used :type Boolean))
  (return true))

(fn `UserConstructionScript`
  (`SphereComponent.SetSphereRadius` (`self.InteractTrigger`) (`self.InteractRadius`) true))