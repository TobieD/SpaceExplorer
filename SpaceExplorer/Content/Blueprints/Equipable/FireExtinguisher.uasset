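; Equipable fire extinguisher that puts out fires on ship tiles.
; Use fires a short burst of the Extinguisher effect, switched off by timer, then runs a visibility line trace between the points from Positions, optionally drawn for debugging.
; If the trace hits a ShipTile, it calls ExtinguishFire on that tile and then the parent Use; otherwise it stops after the trace.
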(event `self.ReceiveBeginPlay`
  (`parent.ReceiveBeginPlay`))

(event `self.ReceiveActorBeginOverlap`
  (params (OtherActor :type "Actor Object Reference")))

(event `self.ReceiveTick`
  (params (DeltaSeconds :type "Float (single-precision)")))

(fn `Debug Linetrace`
  (returns (ReturnValue :type "KismetSystemLibrary.EDrawDebugTrace Enum"))
  (return (select `bool` (`self.Debug`) :`true` "ForDuration" :!type "KismetSystemLibrary.EDrawDebugTrace Enum")))

(fn `Use`
  (returns (used :type Boolean))
  (bind _returnvalue (`SceneComponent.GetSocketLocation` "Nozzle"))
  (bind _check_range (`self.Check Range`))
  (`ActorComponent.Activate` (`self.Extinguisher`) true)
  (`KismetSystemLibrary.K2_SetTimer` (`self.Extinguisher`) "Deactivate" 0.7)
  (bind _outhit (`KismetSystemLibrary.LineTraceSingle` :`Start` _returnvalue :`End` (+ _returnvalue (+ (* (`KismetMathLibrary.GetForwardVector` (`self.K2_GetActorRotation` (`self.Equip Actor`))) (`KismetMathLibrary.MakeVector` _check_range _check_range 0.0)) (0.0 0.0 -100.0))) :`TraceChannel` "TraceTypeQuery1" :`DrawDebugType` (`self.Debug Linetrace`)))
  (bind _asship_tile (cast `/Game/Blueprints/Ship/Generation/ShipTile` (`.HitActor` (`GameplayStatics.BreakHitResult` _outhit))))
  (`/Game/Blueprints/Ship/Generation/ShipTile.Extinguish Fire` _asship_tile)
  (`parent.Use`)
  (return false))

(fn `UserConstructionScript`
  (`parent.UserConstructionScript`))