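; MedicSystem is a ship system that heals crew members near its workstation while it is being worked.
; Start and finish working events toggle the Burst effect and a looping timer that calls Work.
; Work checks the parent ship's CrewList by distance to the workstation and passes nearby members to RestoreCrewHealth.
; Healing adds the ship's MedicHealRate plus a level-scaled bonus to current health, with no clamp shown.
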(event Custom|Start%20Working_Event
  (|BeginWork))

(event Custom|Finish%20Working_Event
  (|Endwork))

(event EventBeginPlay
  (Components|Activation|Deactivate (Variables|Default|GetBurst))
  (EventDispatchers|BindEventtoStartWorking (delegate Custom|Start%20Working_Event))
  (EventDispatchers|BindEventtoFinishWorking (delegate Custom|Finish%20Working_Event)))

(fn ConstructionScript
  (|CallParentFunction))

(fn RestoreCrewHealth
  (params (CrewMember :type Base%20Crew%20Member%20Object%20Reference))
  (Utilities|IsValid CrewMember
    (:Is%20Valid
      (Variables|/Game/Blueprints/Character/BaseCrewMember.BaseCrewMember_C|SetCurrent%20Health CrewMember (|curr+(rate+bonus) (Variables|/Game/Blueprints/Character/BaseCrewMember.BaseCrewMember_C|GetCurrent%20Health CrewMember) (Variables|/Game/Blueprints/Ship/Ship.Ship_C|GetMedic%20Heal%20Rate (Variables|/Game/Blueprints/Character/BaseCrewMember.BaseCrewMember_C|GetParent%20Ship CrewMember)) (Variables|Default|GetBonus%20heal%20rate)))
      (Development|PrintString "Healing"))))

(fn ChangeLevel
  (params (Is%20upgrade :type Boolean))
  (|CallParentFunction Is%20upgrade)
  (Variables|Default|SetBonus%20heal%20rate (* (Variables|Default|GetCurrent%20Level) 2.0))
  (return false))

(fn Work
  (bind _workstation (Variables|Default|GetWorkStation))
  (bind _parent_ship (Variables|/Game/Blueprints/Ship/Walls/BaseInteractable.BaseInteractable_C|GetParent%20Ship _workstation))
  (Utilities|IsValid _parent_ship
    (:Is%20Valid
      ;[0.09557 0.7282 1] Go through all Crewmembers of the ship
      (for _array_element (Variables|/Game/Blueprints/Ship/Ship.Ship_C|GetCrewList _parent_ship)
        (if (Utilities|IsNear (Variables|Default|GetDistance) (Transformation|GetActorLocation _array_element) (Transformation|GetActorLocation (Variables|Default|GetWorkStation)))
          (CallFunction|RestoreCrewHealth _array_element))
        (return)))
    (:Is%20Not%20Valid
      _))
  (return))