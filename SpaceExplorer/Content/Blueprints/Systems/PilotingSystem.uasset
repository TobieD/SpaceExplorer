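; PilotingSystem is a ship system that shows the travel map while it is being worked and boosts the player ship's engine recharge.
; The Piloting_UI widget is created on first work start, cached as TravelMap, then added to or removed from the viewport as work starts and finishes.
; ChangeLevel sets BonusEngineRecharge proportional to CurrentLevel before calling the parent implementation.
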(event `Start Working_Event`
  ;[1 0.9141 0.25] Create UI First Time behaviour is called
  (if (not (`self.CreatedUI`))
    (set `self.CreatedUI` true)
    (bind _returnvalue (`|CreateWidget` "/Game/Blueprints/HUD/PlayerShip/Piloting_UI.Piloting_UI_C"))
    (set `self.TravelMap` _returnvalue))
  (`UserWidget.AddToViewport` (`self.TravelMap`) 0))

(event `Finish Working_Event`
  (`Widget.RemoveFromParent` (`self.TravelMap`)))

(fn `ChangeLevel`
  (params (`Is upgrade` :type Boolean))
  (returns (Changed :type Boolean))
  (set `/Game/Blueprints/Ship/Ship.Bonus Engine Recharge` (* (`self.Current Level`) 0.2) (`/Game/Blueprints/General/Helpers.Get Player Ship`))
  (bind _changed (`parent.ChangeLevel` `Is upgrade`))
  (return _changed))

(fn `UserConstructionScript`
  (`parent.UserConstructionScript`))