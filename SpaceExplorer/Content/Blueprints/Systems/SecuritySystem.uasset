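; Security System is an upgradable ship system that controls how Door actors behave at each level.
; On a level change, it applies the current level to every Door in the world, found once and cached without filtering by ship.
; Level 0 makes doors automated and indestructible, level 1 enables interaction and destruction, and higher levels update their max hits through DestroyableComponent.
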(event `Start Working_Event`)

(event `Finish Working_Event`)

(fn `ChangeLevel`
  (params (`Is upgrade` :type Boolean))
  (returns (Changed :type Boolean))
  (`parent.ChangeLevel` `Is upgrade`)
  (`|ExecutionSequence`
    (:`then_0`
      (if (<= (`self.Current Level`) 1)
        (for _array_element (`self.Get Ship Doors`)
          (switch `int` (`self.Current Level`)
            (:`0`
              (set `/Game/Blueprints/Ship/Walls/BaseInteractable.AllowInteraction` false _array_element)
              (set `/Game/Blueprints/Components/DestroyableComponent.Enabled` false (`/Game/Blueprints/Ship/Walls/Door.DestroyableComponent` _array_element)))
            (:`1`
              (set `/Game/Blueprints/Ship/Walls/BaseInteractable.AllowInteraction` true _array_element)
              (set `/Game/Blueprints/Components/DestroyableComponent.Enabled` true (`/Game/Blueprints/Ship/Walls/Door.DestroyableComponent` _array_element)))))
        (else
          (for _array_element_2 (`self.Get Ship Doors`)
            (`/Game/Blueprints/Components/DestroyableComponent.Update Max Hits` (`/Game/Blueprints/Ship/Walls/Door.DestroyableComponent` _array_element_2) (`KismetMathLibrary.Conv_IntToDouble` (- (`self.Current Level`) 2)))))))
    (:`then_1`
      (return false))))

(fn `Get Ship Doors`
  (returns (`Ship doors` :type "Array of /Game/Blueprints/Ship/Walls/Door Object Reference"))
  (if (<= (`KismetArrayLibrary.Array_Length` (`self.ShipDoors`)) 0)
    ;[0.09557 0.7282 1] Find All Door actors in the world
    (bind _outactors (`GameplayStatics.GetAllActorsOfClass` "/Game/Blueprints/Ship/Walls/Door.Door_C"))
    (for _array_element _outactors
      ;[0.09557 0.7282 1] Store the doors for later
      (`KismetArrayLibrary.Array_Add` (`self.ShipDoors`) _array_element)))
  (return (`self.ShipDoors`)))

(fn `UserConstructionScript`
  (`parent.UserConstructionScript`))