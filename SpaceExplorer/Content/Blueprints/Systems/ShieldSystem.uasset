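; Ship shield system that activates the parent ship's shields while its workstation is being worked and regenerates them over time.
; Starting work restores shields immediately, then on a looping WorkTick timer, adding ship rate plus level-scaled bonus, clamped to maximum.
; It also runs an experience timer; finishing work deactivates shields and clears that timer, but not the looping restore timer.
; ChangeLevel extends the parent's version to recompute the bonus from CurrentLevel.
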(event `Start Working_Event`
  ;[0.09557 0.7282 1] Enable Shields for the ship
  (set `/Game/Blueprints/Ship/Ship.ShieldActive` true (`/Game/Blueprints/Ship/Walls/BaseInteractable.Parent Ship` (`self.WorkStation`)))
  (`KismetSystemLibrary.K2_SetTimerDelegate` (delegate `Working_Event`) (`self.WorkTick`) true)
  (`self.Start Experience Timer`)
  (`self.RestoreShields`))

(event `Finish Working_Event`
  ;[0.09557 0.7282 1] Disable shields for the ship
  (set `/Game/Blueprints/Ship/Ship.ShieldActive` false (`/Game/Blueprints/Ship/Walls/BaseInteractable.Parent Ship` (`self.WorkStation`)))
  (`self.Clear Experience Timer`))

(event `Working_Event`
  (`self.RestoreShields`))

(fn `ChangeLevel`
  (params (`Is upgrade` :type Boolean))
  (returns (Changed :type Boolean))
  (`parent.ChangeLevel` false)
  (set `self.Bonus Restore Rate` (* (`self.Current Level`) 2.0))
  (return false))

(fn `RestoreShields`
  (bind _parent_ship (`/Game/Blueprints/Ship/Walls/BaseInteractable.Parent Ship` (`self.WorkStation`)))
  ;[1 0.1 0.1] Check if ship has full shields
  (bind _fullshield (`/Game/Blueprints/Ship/Ship.HasFullShields` _parent_ship))
  (if (not _fullshield)
    (set `/Game/Blueprints/Ship/Ship.Current Shield ` (`KismetMathLibrary.FClamp` (+ (`/Game/Blueprints/Ship/Ship.Current Shield ` _parent_ship) (+ (`/Game/Blueprints/Ship/Ship.Shield Restore Rate` _parent_ship) (`self.Bonus Restore Rate`))) 0.0 (`/Game/Blueprints/Ship/Ship.Max Shield` _parent_ship)) _parent_ship)
    (return)))

(fn `UserConstructionScript`
  (`parent.UserConstructionScript`))