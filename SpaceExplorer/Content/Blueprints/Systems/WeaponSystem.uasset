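; Ship system for a weapons workstation that lets the player aim equipped weapons at the enemy ship.
; When work starts with an active enemy ship, it hides that ship's ceiling, blends to the enemy ship camera and turns on target finding for every equipped weapon.
; Finishing reverts this and frees workstation movement, while an experience timer runs during use.
; Level changes scale the bonus cooldown restore rate with current level.
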(event `Start Working_Event`
  (bind _enemy_ship (`/Game/Blueprints/General/Helpers.Get Enemy Ship`))
  (`self.Start Experience Timer`)
  (if (`/Game/Blueprints/Ship/EnemyShip.Is Active` _enemy_ship)
    (`/Game/Blueprints/Ship/EnemyShip.Switch Ceiling` _enemy_ship false)
    (`PlayerController.SetViewTargetWithBlend` (`GameplayStatics.GetPlayerController` 0) (`/Game/Blueprints/General/Helpers.Get Enemy Ship Camera`) 0.0 "VTBlend_Linear" 0.0 false)
    (for _array_element (`/Game/Blueprints/Weapons/WeaponCollection.EquipedWeapons` (`/Game/Blueprints/Ship/Ship.WeaponSystem` (`/Game/Blueprints/General/Helpers.Get Player Ship`)))
      (set `/Game/Blueprints/Weapons/BaseWeapon.FindTarget` true _array_element))))

(event `Finish Working_Event`
  (`self.Clear Experience Timer`)
  (`/Game/Blueprints/Ship/EnemyShip.Switch Ceiling` (`/Game/Blueprints/General/Helpers.Get Enemy Ship`) true)
  (for _array_element (`/Game/Blueprints/Weapons/WeaponCollection.EquipedWeapons` (`/Game/Blueprints/Ship/Ship.WeaponSystem` (`/Game/Blueprints/General/Helpers.Get Player Ship`)))
    (set `/Game/Blueprints/Weapons/BaseWeapon.FindTarget` false _array_element))
  (`PlayerController.SetViewTargetWithBlend` (`GameplayStatics.GetPlayerController` 0) (`GameplayStatics.GetPlayerCharacter` 0) 0.0 "VTBlend_Linear" 0.0 false)
  (`/Game/Blueprints/Ship/Interactables/WorkStation.Allow Movement` (`self.WorkStation`) true))

(fn `ChangeLevel`
  (params (`Is upgrade` :type Boolean))
  (returns (Changed :type Boolean))
  (`parent.ChangeLevel` false)
  (set `self.Bonus Cooldown restore rate` (* (`self.Current Level`) 0.2))
  (return true))

(fn `UserConstructionScript`
  (`parent.UserConstructionScript`))