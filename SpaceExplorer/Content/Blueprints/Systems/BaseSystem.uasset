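; Base Blueprint for ship systems that can be worked and leveled with the player ship's skillpoints.
; Starting work runs a looping timer into an empty Working event and a second timer that periodically grants the player ship experience; finishing work clears only the experience timer.
; Adding or removing a level spends or refunds a skillpoint within level limits, then calls ChangeLevel, which shows a notification and serves as the hook for system-specific adjustments.
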(event `Start Working_Event`
  ;[1 1 1] Start Event Linked to Working + experience timer
  (`KismetSystemLibrary.K2_SetTimerDelegate` (delegate `Working_Event`) (`self.WorkTick`) true)
  (`self.Start Experience Timer`))

(event `Working_Event`)

(event `Finish Working_Event`
  ;[1 1 1] Stop Gaining Experience
  (`self.Clear Experience Timer`))

(fn `Add Level`
  (bind _player_ship (`/Game/Blueprints/General/Helpers.Get Player Ship`))
  ;[1 0.1 0.1] Have enough to spend
  (bind _able_to_spend (`/Game/Blueprints/Ship/PlayerShip.Can Spend Skillpoint` _player_ship))
  (if _able_to_spend
    (if (< (`self.Current Level`) (`self.Max Level`))
      (`/Game/Blueprints/Ship/PlayerShip.Spend Skillpoint` _player_ship)
      ;[0.2884 0.68 0.2152] Level up system
      (set `self.Current Level` (`KismetMathLibrary.Clamp` (+ (`self.Current Level`) 1) 0 (`self.Max Level`)))
      (`self.ChangeLevel` true))))

(fn `ChangeLevel`
  (params (`Is upgrade` :type Boolean :default false))
  (returns (Changed :type Boolean))
  (`/Game/Blueprints/General/Helpers.Notify` (`self.Level Text` `Is upgrade`) 1.0)
  (return true))

(fn `Clear Experience Timer`
  (`KismetSystemLibrary.K2_ClearTimer` null "Grant Experience"))

(fn `Grant Experience`
  (bind _asbase_crew_member (cast `/Game/Blueprints/Character/BaseCrewMember` (`GameplayStatics.GetPlayerCharacter` 0)))
  (bind _asplayer_ship (cast `/Game/Blueprints/Ship/PlayerShip` (`/Game/Blueprints/Character/BaseCrewMember.Parent Ship` _asbase_crew_member)))
  (`/Game/Blueprints/Ship/PlayerShip.Grant Experience` _asplayer_ship 5.0))

(fn `Remove Level`
  (if (> (`self.Current Level`) 0)
    (`/Game/Blueprints/Ship/PlayerShip.Grant Skillpoint` (`/Game/Blueprints/General/Helpers.Get Player Ship`))
    ;[0.2884 0.68 0.2152] Change level + call level change event to adjust specific systems
    (set `self.Current Level` (`KismetMathLibrary.Clamp` (- (`self.Current Level`) 1) 0 (`self.Max Level`)))
    (`self.ChangeLevel` false)))

(fn `Start Experience Timer`
  (`KismetSystemLibrary.K2_SetTimer` null "Grant Experience" 15.0 true))

(fn `UserConstructionScript`)