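; Helper function library for an FTL-style ship game, giving shared access to game state, HUD, ships, notifications and score.
; Getters cast to the FTL game state and return its validity-checked player HUD, player and enemy ships, and enemy ship camera.
; Notify shows an on-screen message and also pushes a new widget to the HUD's notification stack.
; Other utilities add score on the standard game mode and pick random actor transforms or texts from lists.
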(fn Notify
  (params (Text :type Text) (Duration :type Float%20%28single-precision%29 :default 0.0) (Type :type ENotificationType%20Enum :default "NewEnumerator0"))
  ;[0.3077 1 0.2929] Store locally
  (LocalVariables|Settext_l Text)
  (LocalVariables|Setduration_l Duration)
  (LocalVariables|Settype_l Type)
  ;[0.2699 0.5609 1] Push notification to screen
  (Default|Notify (Variables|/Game/Blueprints/HUD/Game_UI.Game_UI_C|GetNotification (QualityofLife|GetHUD)) (LocalVariables|Gettext_l) (LocalVariables|Getduration_l) (LocalVariables|Gettype_l))
  ;[0.2699 0.5609 1] Push to stack
  (bind _returnvalue (UserInterface|CreateWidget "/Game/Blueprints/HUD/NotificationSystem/Notification_UI.Notification_UI_C" 0 (LocalVariables|Gettext_l) (LocalVariables|Gettype_l)))
  (Default|NewNotification (Variables|/Game/Blueprints/HUD/Game_UI.Game_UI_C|GetNotificationStack (QualityofLife|GetHUD)) _returnvalue))

(fn GetGameStateFTL
  (bind _asgame_state_ftl (Utilities|Casting|CastToGameState_Ftl (Game|GetGameState)))
  (Utilities|IsValid _asgame_state_ftl
    (:Is%20Valid
      (return _asgame_state_ftl))))

(fn GetGameModeFTL
  (bind _asstandard_game_mode (Utilities|Casting|CastToStandard_GameMode (Game|GetGameMode)))
  (return _asstandard_game_mode))

(fn GetHUD
  (bind _returnvalue (Game|GetPlayerCharacter 0))
  (bind _game_state (QualityofLife|GetGameStateFTL _returnvalue))
  (bind _playerhud (Variables|/Game/Blueprints/General/GameState_Ftl.GameState_Ftl_C|GetPlayerHud _game_state))
  (Utilities|IsValid _playerhud
    (:Is%20Valid
      (return _playerhud))))

(fn GetPlayerShip
  (bind _returnvalue (Game|GetPlayerCharacter 0))
  (bind _game_state (QualityofLife|GetGameStateFTL _returnvalue))
  (bind _playership (Variables|/Game/Blueprints/General/GameState_Ftl.GameState_Ftl_C|GetPlayerShip _game_state))
  (Utilities|IsValid _playership
    (:Is%20Valid
      (return _playership))))

(fn GetEnemyShip
  (bind _returnvalue (Game|GetPlayerCharacter 0))
  (bind _game_state (QualityofLife|GetGameStateFTL _returnvalue))
  (bind _enemyship (Variables|/Game/Blueprints/General/GameState_Ftl.GameState_Ftl_C|GetEnemyShip _game_state))
  (Utilities|IsValid _enemyship
    (:Is%20Valid
      (return _enemyship))))

(fn GetEnemyShipCamera
  (bind _returnvalue (Game|GetPlayerCharacter 0))
  (bind _game_state (QualityofLife|GetGameStateFTL _returnvalue))
  (bind _enemyshipcamera (Variables|/Game/Blueprints/General/GameState_Ftl.GameState_Ftl_C|GetEnemyShipCamera _game_state))
  (Utilities|IsValid _enemyshipcamera
    (:Is%20Valid
      (return _enemyshipcamera))))

(fn RandomTransformfromList
  (params (Actor%20Array :type Array%20of%20Actor%20Object%20References))
  (bind _output_get (LocalVariables|Setarray Actor%20Array))
  (return (Transformation|GetActorTransform (Utilities|Array|Get(acopy) (LocalVariables|Getarray) (Math|Random|RandomInteger (Utilities|Array|Length _output_get))))))

(fn RandomTextfromList
  (params (Text%20List :type Array%20of%20Texts))
  (return (Utilities|Array|Get(acopy) Text%20List (Math|Random|RandomInteger (Utilities|Array|Length Text%20List)))))

(fn AddScore
  (params (Value :type Integer :default 0))
  (bind _returnvalue (Game|Player|GetPlayerPawn 0))
  (bind _game_mode (QualityofLife|GetGameModeFTL _returnvalue))
  (Variables|/Game/Blueprints/General/Standard_GameMode.Standard_GameMode_C|SetScore _game_mode (+ Value (Variables|/Game/Blueprints/General/Standard_GameMode.Standard_GameMode_C|GetScore _game_mode))))