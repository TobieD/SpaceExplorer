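; Standard game mode Blueprint that handles the win and lose end states of a match.
; Both the Win and Lose events pause the game and add a GameEndMenu_UI widget to the viewport, passing it the outcome text and the score from GetGameModeFTL.
; Win also awards a bonus through AddScore before showing the menu, while Lose prints a message after showing it.
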(event `Lose`
  (`GameplayStatics.SetGamePaused` true)
  (bind _returnvalue (`|CreateWidget` "/Game/Blueprints/HUD/GameEndMenu_UI.GameEndMenu_UI_C" null "You lost" (`/Game/Blueprints/General/Standard_GameMode.Score` (`/Game/Blueprints/General/Helpers.Get Game Mode FTL`))))
  (`UserWidget.AddToViewport` _returnvalue 0)
  (`KismetSystemLibrary.PrintString` "Lost"))

(event `Win`
  (`/Game/Blueprints/General/Helpers.Add Score` 200)
  (`GameplayStatics.SetGamePaused` true)
  (bind _returnvalue (`|CreateWidget` "/Game/Blueprints/HUD/GameEndMenu_UI.GameEndMenu_UI_C" null "Won" (`/Game/Blueprints/General/Standard_GameMode.Score` (`/Game/Blueprints/General/Helpers.Get Game Mode FTL`))))
  (`UserWidget.AddToViewport` _returnvalue 0))

(fn `UserConstructionScript`)