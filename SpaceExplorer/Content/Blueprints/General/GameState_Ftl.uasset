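; GameState Blueprint that manages pausing and unpausing the game along with the matching UI.
; On BeginPlay it runs a console command to disable all on-screen messages.
; PauseGame pauses the game, adds PauseUI to the viewport and removes PlayerHud; UnpauseGame reverses this swap.
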(event `self.ReceiveBeginPlay`
  (`KismetSystemLibrary.ExecuteConsoleCommand` "DisableAllScreenMessages"))

(fn `Pause Game`
  (`GameplayStatics.SetGamePaused` true)
  (`UserWidget.AddToViewport` (`self.Pause UI`) 0)
  (`Widget.RemoveFromParent` (`self.PlayerHud`)))

(fn `Unpause Game`
  (`GameplayStatics.SetGamePaused` false)
  (`Widget.RemoveFromParent` (`self.Pause UI`))
  (`UserWidget.AddToViewport` (`self.PlayerHud`) 0))

(fn `UserConstructionScript`)