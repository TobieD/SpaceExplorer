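; Fire tile-state Blueprint that burns crew members and spreads fire to other ship tiles.
; ActivateFire and DeactivateFire toggle the active flag and particles, and control sound and the SpreadableComponent tied to the parent tile.
; Actors found by that component have their ShipTile state changed.
; Collider overlaps, gated by an active check, start and clear a looping timer that damages a single stored crew Target and flags it as in fire.
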(event `self.ReceiveBeginPlay`
  (add `/Game/Blueprints/Components/SpreadableComponent.FoundActor` (`self.SpreadableComponent`) (delegate `OnSpread`)))

(event `OnSpread`
  (params (`Found Actor` :type "Actor Object Reference"))
  (bind _asship_tile (cast `/Game/Blueprints/Ship/Generation/ShipTile` `Found Actor`))
  (`/Game/Blueprints/Ship/Generation/ShipTile.Set Tile State` _asship_tile "NewEnumerator1"))

(event `self.Collider.OnComponentBeginOverlap`
  (params (OtherActor :type "Actor Object Reference") (OtherComp :type "PrimitiveComponent Object Reference") (OtherBodyIndex :type Integer) (bFromSweep :type Boolean) (SweepResult :type "EngineTypes.HitResult Structure (by ref)"))
  (`self.Is Fire Active`)
  (bind _asbase_crew_member (cast `/Game/Blueprints/Character/BaseCrewMember` OtherActor))
  (set `self.Target` _asbase_crew_member)
  (`KismetSystemLibrary.K2_SetTimer` null "FireDamage" 0.4 true))

(event `self.Collider.OnComponentEndOverlap`
  (params (OtherActor :type "Actor Object Reference") (OtherComp :type "PrimitiveComponent Object Reference") (OtherBodyIndex :type Integer))
  (`self.Is Fire Active`)
  (`KismetSystemLibrary.K2_ClearTimer` null "FireDamage")
  (set `/Game/Blueprints/Character/BaseCrewMember.IsInFire` false (`self.Target`)))

(fn `ActivateFire`
  (bind _parent_tile (`self.Parent Tile`))
  (bind _spreadablecomponent (`self.SpreadableComponent`))
  (set `self.IsActive` true)
  (`ActorComponent.Activate` (`self.FireEmitter`) true)
  ;[0.09557 0.7282 1] Set up spreadable Component
  (`/Engine/EditorBlueprintResources/StandardMacros.IsValid` _parent_tile
    (:`Is Valid`
      (set `/Game/Blueprints/Components/SpreadableComponent.Parent` _parent_tile _spreadablecomponent)
      (`/Game/Blueprints/Components/SpreadableComponent.Start` _spreadablecomponent)
      (`AudioComponent.Play` (`self.FireSound`) 0.0))))

(fn `DeactivateFire`
  (bind _target (`self.Target`))
  (bind _spreadablecomponent (`self.SpreadableComponent`))
  (`KismetSystemLibrary.K2_ClearTimer` null "FireDamage")
  (set `self.IsActive` false)
  ;[1 0.7855 0.2499] Stop the particle
  (`ActorComponent.Deactivate` (`self.FireEmitter`))
  ;[0.2699 0.5609 1] Stop Spreading
  (`/Engine/EditorBlueprintResources/StandardMacros.IsValid` _spreadablecomponent
    (:`Is Valid`
      (`/Game/Blueprints/Components/SpreadableComponent.Stop` _spreadablecomponent)
      (`AudioComponent.Stop` (`self.FireSound`))
      (`/Engine/EditorBlueprintResources/StandardMacros.IsValid` _target
        (:`Is Valid`
          (set `/Game/Blueprints/Character/BaseCrewMember.IsInFire` false _target))))))

(fn `FireDamage`
  (bind _target (`self.Target`))
  (set `/Game/Blueprints/Character/BaseCrewMember.IsInFire` true _target)
  (`/Game/Blueprints/Character/BaseCrewMember.TakeDamage_Event` _target 3.0))

(fn `UserConstructionScript`)